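; Spawner actor that builds the endless tunnel from BP_Tunnel segments and populates each with enemies and pickups.
; On BeginPlay it destroys existing tunnels, then chains new ones from the player's location via each segment's SpawnPoint.
; Each segment gets a randomized wall, usually Manhacks, and occasionally health or invincibility pickups, attached at random child spawn points.
; Each tunnel receives a spawner reference, and SpawnTunnelAtPoint extends the chain from the newest one.
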(event EventBeginPlay
  (CallFunction|SpawnInitTunnels))

(event Collision|EventActorBeginOverlap
  (params (OtherActor :type Actor%20Object%20Reference)))

(event EventTick
  (params (DeltaSeconds :type Float%20%28single-precision%29)))

(fn ConstructionScript)

(fn SpawnTunnel
  (params (SpawnLoc :type Vector))
  (bind _returnvalue (Game|SpawnActorfromClass "/Game/InfiniteMatrix/Blueprints/BP_Tunnel.BP_Tunnel_C" (Math|Transform|MakeTransform SpawnLoc "0, 0, 0" "1.000000,1.000000,1.000000") "Undefined" "MultiplyWithRoot" 0 0))
  (bind _output_get (Variables|Default|SetNewTunnel _returnvalue))
  (Variables|/Game/InfiniteMatrix/Blueprints/BP_Tunnel.BP_Tunnel_C|SetTunnelSpawner _output_get self)
  (Default|RandomWall _output_get)
  (CallFunction|SpawnManhacks _returnvalue)
  (if (== 1 (Math|Random|RandomIntegerinRange 0 7))
    (CallFunction|SpawnHealthPacks _returnvalue))
  (if (== 0 (Math|Random|RandomIntegerinRange 0 5))
    (CallFunction|SpawnPowerup _returnvalue)))

(fn SpawnTunnelatPoint
  (CallFunction|SpawnTunnel (Transformation|GetWorldLocation (Variables|/Game/InfiniteMatrix/Blueprints/BP_Tunnel.BP_Tunnel_C|GetSpawnPoint (Variables|Default|GetNewTunnel)))))

(fn SpawnInitTunnels
  (Utilities|FlowControl|Sequence
    (:then_0
      (bind _outactors (Actor|GetAllActorsOfClass "/Game/InfiniteMatrix/Blueprints/BP_Tunnel.BP_Tunnel_C"))
      (for _array_element _outactors
        (Actor|DestroyActor _array_element)))
    (:then_1
      (for _index (range 0 2)
        (Utilities|IsValid (Variables|Default|GetNewTunnel)
          (:Is%20Valid
            (CallFunction|SpawnTunnelatPoint))
          (:Is%20Not%20Valid
            (CallFunction|SpawnTunnel (Transformation|GetActorLocation (Game|Player|GetPlayerPawn 0)))))))))

(fn SpawnHealthPacks
  (params (ParentTunnel :type BP%20Tunnel%20Object%20Reference))
  (bind _returnvalue (Game|SpawnActorfromClass "/Game/InfiniteMatrix/Blueprints/BP_HealthPack.BP_HealthPack_C" (Math|Transform|MakeTransform (Transformation|GetWorldLocation (.Random%20Element (Utilities|GetRandomArrayElement (Components|GetChildrenComponents (Variables|/Game/InfiniteMatrix/Blueprints/BP_Tunnel.BP_Tunnel_C|GetHP_SpawnPoints ParentTunnel) false))))) "AdjustIfPossibleButAlwaysSpawn" "MultiplyWithRoot" 0 0))
  (Transformation|AttachActorToActor _returnvalue ParentTunnel "None" "KeepWorld" "KeepWorld" "KeepWorld" true)
  (return 0))

(fn SpawnManhacks
  (params (ParentTunnel :type BP%20Tunnel%20Object%20Reference))
  (bind _returnvalue (Math|Random|RandomIntegerinRange 0 9))
  (bind _enemy_spawnpoints (Variables|/Game/InfiniteMatrix/Blueprints/BP_Tunnel.BP_Tunnel_C|GetEnemy_SpawnPoints ParentTunnel))
  (bind _children (Components|GetChildrenComponents _enemy_spawnpoints false))
  (if (not (== 0 _returnvalue))
    (if (<= _returnvalue 2) ; if <=, spawn 1 Manhack, if > 7, spawn 2 Manhacks. Maybe 2 and 3 are better amounts (for more challenge)
      (bind _returnvalue_2 (Game|SpawnActorfromClass "/Game/InfiniteMatrix/Blueprints/BP_Manhack.BP_Manhack_C" (Math|Transform|MakeTransform (Transformation|GetWorldLocation (.OutItem (Utilities|Array|Random _children)))) "AdjustIfPossibleButAlwaysSpawn" "MultiplyWithRoot" 0 0))
      (Transformation|AttachActorToActor _returnvalue_2 ParentTunnel "None" "KeepWorld" "KeepWorld" "KeepWorld" true)
      (else
        (bind _output_get (LocalVariables|SetEnemySPs _children))
        (Utilities|Array|Shuffle _output_get)
        (if (<= _returnvalue 6)
          (LocalVariables|SetNumManhacks 2)
          (else
            (LocalVariables|SetNumManhacks 4)))
        (for _index (range 0 (LocalVariables|GetNumManhacks))
          (bind _returnvalue_3 (Game|SpawnActorfromClass "/Game/InfiniteMatrix/Blueprints/BP_Manhack.BP_Manhack_C" (Math|Transform|MakeTransform (Transformation|GetWorldLocation (Utilities|Array|Get(acopy) (LocalVariables|GetEnemySPs) _index))) "AdjustIfPossibleButAlwaysSpawn" "MultiplyWithRoot" 0 0))
          (Transformation|AttachActorToActor _returnvalue_3 ParentTunnel "None" "KeepWorld" "KeepWorld" "KeepWorld" true))))
    (return 0)))

(fn SpawnPowerup
  (params (ParentTunnel :type BP%20Tunnel%20Object%20Reference))
  (bind _returnvalue (Game|SpawnActorfromClass "/Game/InfiniteMatrix/Blueprints/BP_InvincibilityPowerUp.BP_InvincibilityPowerUp_C" (Math|Transform|MakeTransform (Transformation|GetWorldLocation (.OutItem (Utilities|Array|Random (Components|GetChildrenComponents (Variables|/Game/InfiniteMatrix/Blueprints/BP_Tunnel.BP_Tunnel_C|GetPowerup_SpawnPoints ParentTunnel) false))))) "Undefined" "MultiplyWithRoot" 0 0))
  (Transformation|AttachActorToActor _returnvalue ParentTunnel "None" "KeepWorld" "KeepWorld" "KeepWorld" true))