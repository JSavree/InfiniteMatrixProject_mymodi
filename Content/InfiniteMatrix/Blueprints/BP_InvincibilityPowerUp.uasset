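; BP_InvincibilityPowerUp is a pickup that makes the player temporarily invincible.
; On box overlap with a BP_Player that can be damaged, it turns off CanBeDamaged, plays a power-up sound, detaches from its parent and hides.
; After a short delay it plays a power-down sound, restores CanBeDamaged and destroys itself.
; A player who is already invulnerable does not consume it.
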(event OnComponentBeginOverlap(Box)
  (params (OverlappedComponent :type Primitive%20Component%20Object%20Reference) (OtherActor :type Actor%20Object%20Reference) (OtherComp :type Primitive%20Component%20Object%20Reference) (OtherBodyIndex :type Integer) (bFromSweep :type Boolean) (SweepResult :type Hit%20Result%20Structure%20%28by%20ref%29))
  (bind _asbp_player (Utilities|Casting|CastToBP_Player OtherActor))
  (if (Variables|/Script/Engine.Actor|GetbCanBeDamaged _asbp_player)
    (Variables|/Script/Engine.Actor|SetbCanBeDamaged _asbp_player false)
    (Audio|PlaySound2D "/Game/InfiniteMatrix/Audio/220173__gameaudio__spacey-1uppower-up.220173__gameaudio__spacey-1uppower-up" 1.0 1.0 0.0 0 0)
    (Transformation|DetachFromActor "KeepWorld" "KeepWorld" "KeepWorld")
    (Rendering|SetActorHiddenInGame true)
    (Utilities|FlowControl|Delay 4.0)
    (Audio|PlaySound2D "/Game/InfiniteMatrix/Audio/107789__leviclaassen__hit_002_powerdown.107789__leviclaassen__hit_002_powerdown" 1.0 1.0 0.0 0 0)
    (Variables|/Script/Engine.Actor|SetbCanBeDamaged _asbp_player true)
    (Actor|DestroyActor)))

(event EventBeginPlay)

(event Collision|EventActorBeginOverlap
  (params (OtherActor :type Actor%20Object%20Reference)))

(event EventTick
  (params (DeltaSeconds :type Float%20%28single-precision%29)))

(fn ConstructionScript)